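; Arrow projectile actor that deals damage to whatever enemy target, AI character or player its box overlaps.
; On overlap it stops projectile movement, zeroes gravity and casts the hit actor to choose the response.
; Enemy targets are damaged and the arrow is destroyed at once.
; Other hits attach the arrow in place, disable its collision and destroy it after a short delay, damaging only characters.
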(event `self.Box.OnComponentBeginOverlap`
  (params (OverlappedComponent :type "PrimitiveComponent Object Reference") (OtherActor :type "Actor Object Reference") (OtherComp :type "PrimitiveComponent Object Reference") (OtherBodyIndex :type Integer) (bFromSweep :type Boolean) (SweepResult :type "HitResult Structure (by ref)"))
  (bind _box (`self.Box`))
  (bind _projectilemovement (`self.ProjectileMovement`))
  (bind _damage (`self.Damage`))
  (bind _box_2 (`self.Box`))
  (bind _box_3 (`self.Box`))
  (if (!= OtherActor self)
    (`MovementComponent.StopMovementImmediately` _projectilemovement)
    (set `ProjectileMovementComponent.ProjectileGravityScale` 0.0 _projectilemovement)
    (bind _asbp_enemy_target (cast `/Game/Blueprints/Enemy/BP_EnemyTarget` OtherActor)
      (:`then`
        (`GameplayStatics.ApplyDamage` _asbp_enemy_target _damage)
        (`self.K2_DestroyActor`))
      (:`CastFailed`
        (bind _asbp_aicharacter (cast `/Game/Blueprints/Enemy/EnemyAI/BP_AICharacter` OtherActor)
          (:`then`
            (`GameplayStatics.ApplyDamage` _asbp_aicharacter _damage)
            (`self.K2_AttachToActor` OtherActor "None" "KeepWorld" "KeepWorld" "KeepWorld")
            (`/Engine/EditorBlueprintResources/StandardMacros.IsValid` _box
              (:`Is Valid`
                (`PrimitiveComponent.SetCollisionEnabled` _box "NoCollision")
                (`KismetSystemLibrary.Delay` 0.5)
                (`self.K2_DestroyActor`))))
          (:`CastFailed`
            (bind _asbp_player (cast `/Game/Blueprints/Player/BP_Player` OtherActor)
              (:`then`
                (`GameplayStatics.ApplyDamage` _asbp_player _damage)
                (`self.K2_AttachToActor` OtherActor "None" "KeepWorld" "KeepWorld" "KeepWorld")
                (`/Engine/EditorBlueprintResources/StandardMacros.IsValid` _box_3
                  (:`Is Valid`
                    (`PrimitiveComponent.SetCollisionEnabled` _box_3 "NoCollision")
                    (`KismetSystemLibrary.Delay` 0.5)
                    (`self.K2_DestroyActor`))))
              (:`CastFailed`
                (`self.K2_AttachToActor` OtherActor "None" "KeepWorld" "KeepWorld" "KeepWorld")
                (`/Engine/EditorBlueprintResources/StandardMacros.IsValid` _box_2
                  (:`Is Valid`
                    (`PrimitiveComponent.SetCollisionEnabled` _box_2 "NoCollision")
                    (`KismetSystemLibrary.Delay` 1.0)
                    (`self.K2_DestroyActor`)))))))))))

(fn `UserConstructionScript`)