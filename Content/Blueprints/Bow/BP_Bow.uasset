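; Bow weapon Blueprint that extends a parent's shooting behavior to fire arrows.
; OnShoot calls the parent, spawns a BP_FlyingArrow at the given start position, calls ApplyDamage immediately with no target shown, and prints a display name.
; AdjustableShotDistance adds a modifier to the stored projectile distance and returns it, so repeated calls accumulate.
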(fn `AdjustableShotDistance`
  (returns (ShotDistance :type "Float (double-precision)"))
  (bind _output_get (set `self.ProjectileDistance` (+ (`self.ProjectileDistance`) (`self.ProjectileDistanceModifier`))))
  (return _output_get))

(fn `OnShoot`
  (params (StartPosition :type "Transform Structure"))
  (locals (isHeld :type Boolean))
  (`parent.OnShoot` StartPosition)
  (`|SpawnActorFromClass` "/Game/Blueprints/Arrow/BP_FlyingArrow.BP_FlyingArrow_C" StartPosition "AdjustIfPossibleButAlwaysSpawn" "MultiplyWithRoot" null null)
  (`GameplayStatics.ApplyDamage` null (`self.Damage`))
  (`KismetSystemLibrary.PrintString` (`KismetSystemLibrary.GetDisplayName` null)))

(fn `UserConstructionScript`
  (`parent.UserConstructionScript`))