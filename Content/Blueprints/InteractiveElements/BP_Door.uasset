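; BP_Door is an interactive door that slides open along its local Y axis.
; OpenDoor stores the current relative Y, sets a fixed target offset, and plays a Timeline whose Alpha linearly eases the door mesh between them.
; CloseDoor is an empty event; logic to return the door to zero exists but is disconnected, so it never runs.
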(event `OpenDoor`
  (bind (_relativelocation_x _relativelocation_y) (`KismetMathLibrary.BreakVector` (`SceneComponent.RelativeLocation` (`self.Door`))))
  (set `self.CurrentLocation` _relativelocation_y)
  (set `self.NewLocation` 500.0)
  (bind (_direction _alpha) (`Timeline|Timeline` :!via `PlayFromStart`)
    (:`Update`
      (`SceneComponent.K2_SetRelativeLocation` (`self.Door`) (`KismetMathLibrary.MakeVector` 0.0 (`|EaseFunction` "Linear" _alpha (`self.CurrentLocation`) (`self.NewLocation`))) false false))))

(event `CloseDoor`)

(fn `UserConstructionScript`)