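; Health component that tracks an actor's health, with damage, healing, regeneration, death check and normalized value queries.
; BeginPlay initializes max and current health from StartingHealth; Damage and Heal reject negative amounts and route through SetHealth, which clamps to the valid range.
; Tick drives regeneration through a Delay, so HealthRegenRate acts as the seconds between heals and zero or below disables it.
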(event `self.ReceiveBeginPlay`
  (`self.Init` (`self.StartingHealth`)))

(event `self.ReceiveTick`
  (params (DeltaSeconds :type "Float (single-precision)"))
  (if (> (`self.HealthRegenRate`) 0.0)
    (`KismetSystemLibrary.Delay` (`self.HealthRegenRate`))
    (`self.Heal` (`self.HealthRegenAmount`))))

(fn `Damage`
  (params (DamageAmount :type "Float (double-precision)"))
  (if (not (< DamageAmount 0.0))
    (`self.SetHealth` (- (`self.GetHealth`) DamageAmount))))

(fn `GetHealth`
  (returns (Health :type "Float (double-precision)"))
  (return (`self.Health`)))

(fn `GetNormalizedHealth`
  (returns (NormalizedHealth :type "Float (double-precision)"))
  (return (`KismetMathLibrary.FClamp` (/ (`self.Health`) (`self.MaxHealth`)))))

(fn `Heal`
  (params (HealAmount :type "Float (double-precision)"))
  (if (not (< HealAmount 0.0))
    (`self.SetHealth` (+ HealAmount (`self.GetHealth`)))))

(fn `Init`
  (params (MaxHealth :type "Float (double-precision)"))
  (bind _output_get (set `self.MaxHealth` MaxHealth))
  (`self.SetHealth` _output_get))

(fn `IsDead`
  (returns (IsDead :type Boolean))
  (return (<= (`self.GetHealth`) 0.0)))

(fn `SetHealth`
  (params (NewHealth :type "Float (double-precision)"))
  (set `self.Health` (`KismetMathLibrary.FClamp` NewHealth 0.0 (`self.MaxHealth`))))