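; BP_AICharacter is an enemy AI character with health, a health bar widget and helpers for aiming arrows at a target.
; On BeginPlay it creates a WPB_HealthBar for its widget component and registers itself as the owner.
; Damage feeds ACHealthComponent, then either destroys the actor on death or broadcasts normalized health.
; Aiming rotates ArrowSpawnPoint toward the target and scales arrow power linearly with distance.
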(event `self.ReceiveBeginPlay`
  (bind _returnvalue (`|CreateWidget` "/Game/Blueprints/UI/WPB_HealthBar.WPB_HealthBar_C"))
  (`WidgetComponent.SetWidget` (`self.Widget`) _returnvalue)
  (message `/Game/Blueprints/UI/BPI_SetUIOwner.SetUIOwner` _returnvalue null self))

(event `self.ReceiveAnyDamage`
  (params (Damage :type "Float (single-precision)") (DamageType :type "DamageType Object Reference") (InstigatedBy :type "Controller Object Reference") (DamageCauser :type "Actor Object Reference"))
  (`self.TakeDamage` Damage))

(fn `SetArrowDirection`
  (params (target :type "/Game/Blueprints/Player/BP_Player Object Reference"))
  (`SceneComponent.K2_SetWorldRotation` (`self.ArrowSpawnPoint`) (`KismetMathLibrary.FindLookAtRotation` (`self.K2_GetActorLocation` self) (`self.K2_GetActorLocation` target)) false false))

(fn `SetArrowPower`
  (params (Target :type "/Game/Blueprints/Player/BP_Player Object Reference"))
  (returns (ArrowPower :type "Float (double-precision)"))
  (bind _output_get (set `self.Arrow distance` (* 3.0 (`KismetMathLibrary.Vector_Distance` (`self.K2_GetActorLocation` self) (`self.K2_GetActorLocation` Target)))))
  (return _output_get))

(fn `TakeDamage`
  (params (Damage :type "Float (double-precision)"))
  (bind _ac_healthcomponent (`self.AC_HealthComponent`))
  (`/Game/Blueprints/AC_HealthComponent.Damage` _ac_healthcomponent Damage)
  (if (`/Game/Blueprints/AC_HealthComponent.IsDead` _ac_healthcomponent)
    (`self.K2_DestroyActor`)
    (else
      (`self.HealthUpdated` (`/Game/Blueprints/AC_HealthComponent.GetNormalizedHealth` (`self.AC_HealthComponent`))))))

(fn `UserConstructionScript`)